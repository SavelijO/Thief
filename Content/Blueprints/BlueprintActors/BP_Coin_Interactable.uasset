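; BP_Coin_Interactable is a collectible coin that the player picks up by interacting with it.
; On BeginPlay it gets the child actors of its Parent and, if the last one is valid, attaches itself to that actor, keeping its world transform.
; On interact it notifies the coin UI through CollectCoin, then destroys itself.
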(event EventBeginPlay
  (bind _output_get (Variables|Default|SetParentActorArr (Actor|GetAllChildActors (Variables|Default|GetParent) false)))
  (if (Utilities|IsValid (Utilities|Array|Get(acopy) _output_get (- (Utilities|Array|Length _output_get) 1)))
    (Transformation|AttachActorToActor (Utilities|Array|Get(acopy) _output_get (- (Utilities|Array|Length _output_get) 1)) "None" "KeepWorld" "KeepWorld" "KeepWorld" false)))

(event EventOnInteract
  (Default|CollectCoin (Variables|Default|GetCoinUI))
  (Actor|DestroyActor))

(fn ConstructionScript)