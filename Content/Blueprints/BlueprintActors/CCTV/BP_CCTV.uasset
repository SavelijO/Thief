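; BP_CCTV is a security camera actor that visually aims at a detection box and displays an awareness bar.
; Each Tick, it yaws the base with a correction offset and tilts the head using look-at rotations from the actor toward DetectionBox.
; It also turns the awareness bar widget to face the player's capsule.
; BecomeAware and LooseAwarness forward state changes to the BW_Awarness widget; no detection logic lives in this Blueprint.
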(event EventTick
  (params (DeltaSeconds :type Float%20%28single-precision%29))
  (bind _returnvalue (Transformation|GetActorLocation))
  (bind _awarnessbarref (Variables|Default|GetAwarnessBarRef))
  (bind _detection_box (Variables|Default|GetDetection%20Box))
  (bind _returnvalue_2 (Transformation|GetActorLocation _detection_box))
  (bind _returnvalue_3 (Math|Rotator|FindLookatRotation _returnvalue _returnvalue_2))
  (bind (_roll _pitch _yaw) (Math|Rotator|BreakRotator _returnvalue_3))
  (Transformation|SetRelativeRotation (Variables|Default|Getcctv_base) (Math|Rotator|MakeRotator 0.0 0.0 (+ _yaw (Variables|Default|GetCorrectionRotataion))) false false)
  (Transformation|SetRelativeRotation (Variables|Default|Getcctv_head) (Math|Rotator|MakeRotator (* _pitch -1.0) 0.0 0.0) false false)
  (Transformation|SetWorldRotation _awarnessbarref (Math|Rotator|FindLookatRotation (Transformation|GetWorldLocation _awarnessbarref) (Transformation|GetWorldLocation (Variables|/Script/Engine.Character|GetCapsuleComponent (Game|GetPlayerCharacter 0)))) false false))

(fn ConstructionScript)

(fn BecomeAware
  (bind _asbw_awarness (Utilities|Casting|CastToBW_Awarness (UserInterface|GetWidget (Variables|Default|GetAwarnessBarRef))))
  (Default|BecomeAware _asbw_awarness))

(fn LooseAwarness
  (bind _asbw_awarness (Utilities|Casting|CastToBW_Awarness (UserInterface|GetWidget (Variables|Default|GetAwarnessBarRef))))
  (Default|LooseAwarness _asbw_awarness))