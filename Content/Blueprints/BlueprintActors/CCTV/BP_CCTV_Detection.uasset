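; CCTV detection actor that patrols between two points until its trigger overlaps the player, then alerts the CCTV and follows them.
; Tick either snaps it to the player's XY at fixed height or starts a Transition timeline between its current position and the start point.
; That timeline leads into a Patrol timeline lerping from start to end, whose completion lets Tick restart the cycle.
; Nothing here clears the follow flag.
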(event OnComponentBeginOverlap(DetectionTrigger)
  (params (OverlappedComponent :type Primitive%20Component%20Object%20Reference) (OtherActor :type Actor%20Object%20Reference) (OtherComp :type Primitive%20Component%20Object%20Reference) (OtherBodyIndex :type Integer) (bFromSweep :type Boolean) (SweepResult :type Hit%20Result%20Structure%20%28by%20ref%29))
  (if (Actor|ActorHasTag OtherActor "Player")
    (Variables|Default|SetShouldFollowPlayer true)
    (Default|BecomeAware (Variables|Default|GetCCTV))))

(event Custom|Patrol
  (bind _startpos (Variables|Default|GetStartPos))
  (bind _endpos (Variables|Default|GetEndPos))
  (bind (_x _y _z) (Math|Vector|BreakVector _startpos))
  (bind (_x_2 _y_2) (Math|Vector|BreakVector _endpos))
  ;[1 1 1] Patrol
  (Variables|Default|SetIsInTransition false)
  (bind (_direction _xpos _ypos) (Timeline|PatrolPosition PlayFromStart)
    (:Update
      (if (Variables|Default|GetIsOnPatrol)
        (Transformation|SetActorLocation (Math|Vector|MakeVector (Math|Float|Lerp _x _x_2 _xpos) (Math|Float|Lerp _y _y_2 _ypos) _z) false false)
        (else
          (CallFunction|StopTimer))))
    (:Finished
      (Variables|Default|SetIsOnPatrol false)
      (CallFunction|SetNewPatrolTime))))

(event Custom|FollowPlayer
  (bind _returnvalue (Game|GetPlayerCharacter 0))
  (bind _returnvalue_2 (Transformation|GetActorLocation _returnvalue))
  (bind (_x _y) (Math|Vector|BreakVector _returnvalue_2))
  ;[1 1 1] Follow Player
  (Variables|Default|SetIsOnPatrol false)
  (Variables|Default|SetIsInTransition false)
  (Transformation|SetActorLocation (Math|Vector|MakeVector _x _y (.Z (Class|KismetMathLibrary|BreakVector3f (Variables|Default|GetStartPos)))) false false))

(event Custom|StopTimer
  (bind _startpos (Variables|Default|GetStartPos))
  (bind _endpos (Variables|Default|GetEndPos))
  (bind (_x _y _z) (Math|Vector|BreakVector _startpos))
  (bind (_x_2 _y_2) (Math|Vector|BreakVector _endpos))
  ;[1 1 1] Patrol
  (bind (_direction _xpos _ypos) (Timeline|PatrolPosition Stop)
    (:Update
      (if (Variables|Default|GetIsOnPatrol)
        (Transformation|SetActorLocation (Math|Vector|MakeVector (Math|Float|Lerp _x _x_2 _xpos) (Math|Float|Lerp _y _y_2 _ypos) _z) false false)
        (else
          (CallFunction|StopTimer))))
    (:Finished
      (Variables|Default|SetIsOnPatrol false)
      (CallFunction|SetNewPatrolTime))))

(event Custom|SetNewPatrolTime
  (bind _startpos (Variables|Default|GetStartPos))
  (bind _endpos (Variables|Default|GetEndPos))
  (bind (_x _y _z) (Math|Vector|BreakVector _startpos))
  (bind (_x_2 _y_2) (Math|Vector|BreakVector _endpos))
  ;[1 1 1] Patrol
  (bind (_direction _xpos _ypos) (Timeline|PatrolPosition SetNewTime)
    (:Update
      (if (Variables|Default|GetIsOnPatrol)
        (Transformation|SetActorLocation (Math|Vector|MakeVector (Math|Float|Lerp _x _x_2 _xpos) (Math|Float|Lerp _y _y_2 _ypos) _z) false false)
        (else
          (CallFunction|StopTimer))))
    (:Finished
      (Variables|Default|SetIsOnPatrol false)
      (CallFunction|SetNewPatrolTime))))

(event Custom|SetNewTransitionTime
  (bind _startpos (Variables|Default|GetStartPos))
  ;[1 1 1] Transition
  (bind _transition_time (Timeline|Transition SetNewTime)
    (:Update
      (if (Variables|Default|GetIsInTransition)
        (Transformation|SetActorLocation (Math|Vector|MakeVector (Math|Float|Lerp (.x _startpos) (.X (Math|Vector|BreakVector (stale EventTick _output_get))) _transition_time) (Math|Float|Lerp (.y _startpos) (.Y (Math|Vector|BreakVector (stale EventTick _output_get))) _transition_time) (.z _startpos)) false false)))
    (:Finished
      (Variables|Default|SetIsInTransition false)
      (CallFunction|Patrol)
      (CallFunction|SetNewTransitionTime))))

(event EventTick
  (params (DeltaSeconds :type Float%20%28single-precision%29))
  (bind _startpos (Variables|Default|GetStartPos))
  (if (Variables|Default|GetShouldFollowPlayer)
    (CallFunction|FollowPlayer)
    (elif (not (Variables|Default|GetIsOnPatrol))
      ;[1 1 1] Transition
      (Variables|Default|SetIsOnPatrol true)
      (Variables|Default|SetIsInTransition true)
      (bind _output_get (Variables|Default|SetTempPosition (Transformation|GetActorLocation)))
      (bind _transition_time (Timeline|Transition Play)
        (:Update
          (if (Variables|Default|GetIsInTransition)
            (Transformation|SetActorLocation (Math|Vector|MakeVector (Math|Float|Lerp (.x _startpos) (.X (Math|Vector|BreakVector _output_get)) _transition_time) (Math|Float|Lerp (.y _startpos) (.Y (Math|Vector|BreakVector _output_get)) _transition_time) (.z _startpos)) false false)))
        (:Finished
          (Variables|Default|SetIsInTransition false)
          (CallFunction|Patrol)
          (CallFunction|SetNewTransitionTime))))))

(fn ConstructionScript)