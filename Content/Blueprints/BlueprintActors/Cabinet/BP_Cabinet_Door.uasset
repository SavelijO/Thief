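; BP_Cabinet_Door is a cabinet door actor that swings open and closed on interaction.
; OnInteract toggles IsClosed and plays or reverses a timeline, whose Open track lerps the CabinetDoor's relative yaw between zero and Angle.
; Any end overlap on ProximityTrigger also marks the door closed and reverses the timeline, so it shuts automatically without checking which actor left.
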(event OnComponentEndOverlap(ProximityTrigger)
  (params (OverlappedComponent :type Primitive%20Component%20Object%20Reference) (OtherActor :type Actor%20Object%20Reference) (OtherComp :type Primitive%20Component%20Object%20Reference) (OtherBodyIndex :type Integer))
  (Variables|Default|SetIsClosed true)
  (bind _open (Timeline|Timeline Reverse)
    (:Update
      (Transformation|SetRelativeRotation (Variables|Default|Getcabinet_door) (Math|Rotator|MakeRotator 0.0 0.0 (Math|Float|Lerp 0.0 (Variables|Default|GetAngle) _open)) false false))))

(event EventOnInteract
  (if (Variables|Default|GetIsClosed)
    (Variables|Default|SetIsClosed false)
    (bind _open (Timeline|Timeline Play)
      (:Update
        (Transformation|SetRelativeRotation (Variables|Default|Getcabinet_door) (Math|Rotator|MakeRotator 0.0 0.0 (Math|Float|Lerp 0.0 (Variables|Default|GetAngle) _open)) false false)))
    (else
      (Variables|Default|SetIsClosed true)
      (Timeline|Timeline Reverse))))

(fn ConstructionScript)