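; Elevator actor that carries its cabin mesh between floors and operates the cabin and landing doors.
; A button press looks up DesiredFloor in the Floors map, toggles the doors shut if open, then lerps cabin height with the Move timeline.
; Both doors toggle on arrival or a press for the current floor, tracked by IsDoorClosed.
; Leaving the proximity trigger closes any open doors.
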(event OnComponentEndOverlap(Proximitytrigger)
  (params (OverlappedComponent :type Primitive%20Component%20Object%20Reference) (OtherActor :type Actor%20Object%20Reference) (OtherComp :type Primitive%20Component%20Object%20Reference) (OtherBodyIndex :type Integer))
  ;[1 1 1] Close doors on proximity
  (if (not (Variables|Default|GetIsDoorClosed))
    (Default|OnOverlapEndCutom (.FloorDoor (Utilities|Struct|BreakBS_Floor (.Value (Utilities|Map|Find (Variables|Default|GetFloors) (Variables|Default|GetDesiredFloor))))))
    (bind _asbp_elevator_door (Utilities|Casting|CastToBP_Elevator_Door (Variables|/Script/Engine.ChildActorComponent|GetChildActor (Variables|Default|GetBP_Elevator_Door))))
    (Default|OnOverlapEndCutom _asbp_elevator_door)
    (Variables|Default|SetIsDoorClosed true)))

(event Custom|OnButtonPressed
  (bind _fbx_elevevator (Variables|Default|GetFBX_Elevevator))
  (if (not (Variables|Default|GetIsMoving))
    (bind _output_get (Variables|Default|SetCurrent%20Height (.z (.Location (Math|Transform|BreakTransform (Transformation|GetRelativeTransform _fbx_elevevator))))))
    (bind _output_get_2 (Variables|Default|SetDesiredHeight (.FloorHeight (Utilities|Struct|BreakBS_Floor (.Value (Utilities|Map|Find (Variables|Default|GetFloors) (Variables|Default|GetDesiredFloor)))))))
    (if (not (== (Variables|Default|GetDesiredFloor) (Variables|Default|GetCurrentFloor)))
      (Variables|Default|SetIsMoving true)
      (if (Variables|Default|GetIsDoorClosed)
        (Variables|Default|SetCurrentFloor (Variables|Default|GetDesiredFloor))
        (bind _height (Timeline|Move Play)
          (:Update
            (if (Variables|Default|GetIsMoving)
              (Transformation|SetRelativeLocation _fbx_elevevator (Math|Vector|MakeVector 0.0 0.0 (Math|Float|Lerp _output_get _output_get_2 _height)) false false)))
          (:Finished
            (Variables|Default|SetIsMoving false)
            (Utilities|FlowControl|Sequence
              (:then_0
                (CallFunction|InteractwithDoors (Variables|Default|GetCurrentFloor)))
              (:then_1
                (Timeline|Move SetNewTime)))))
        (else
          (CallFunction|InteractwithDoors (Variables|Default|GetCurrentFloor))
          (Utilities|FlowControl|Delay 1.0)
          (Variables|Default|SetCurrentFloor (Variables|Default|GetDesiredFloor))
          (Timeline|Move Play)))
      (else
        (CallFunction|InteractwithDoors (Variables|Default|GetCurrentFloor))))))

(fn ConstructionScript)

(fn InteractwithDoors
  (params (Floor :type Integer))
  (Class|BIInteractable|OnInteract(Message) (Variables|/Script/Engine.ChildActorComponent|GetChildActor (Variables|Default|GetBP_Elevator_Door)))
  (Class|BIInteractable|OnInteract(Message) (.FloorDoor (Utilities|Struct|BreakBS_Floor (.Value (Utilities|Map|Find (Variables|Default|GetFloors) Floor)))))
  (if (Variables|Default|GetIsDoorClosed)
    (Variables|Default|SetIsDoorClosed false)
    (else
      (Variables|Default|SetIsDoorClosed true))))