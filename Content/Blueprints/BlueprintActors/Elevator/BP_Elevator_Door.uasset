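; BP_Elevator_Door is a two-panel sliding elevator door that toggles open and closed on interaction.
; An IsClosed flag decides whether OnInteract plays or reverses the Open timeline, which lerps the two door meshes apart along their relative Y axis.
; A custom overlap-end event sets the flag and reverses the same timeline, closing the door.
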(event Custom|OnOverlapEndCutom
  (Variables|Default|SetIsClosed true)
  (bind _open (Timeline|open Reverse)
    (:Update
      (Transformation|SetRelativeLocation (Variables|Default|GetFBX_Door_Elevator1) (Math|Vector|MakeVector 0.0 (Math|Float|Lerp -158.0 -318.0 _open) 0.0) false false)
      (Transformation|SetRelativeLocation (Variables|Default|GetFBX_Door_Elevator) (Math|Vector|MakeVector 0.0 (Math|Float|Lerp -22.0 138.0 _open) 0.0) false false))))

(event EventOnInteract
  (if (Variables|Default|GetIsClosed)
    (Variables|Default|SetIsClosed false)
    (bind _open (Timeline|open Play)
      (:Update
        (Transformation|SetRelativeLocation (Variables|Default|GetFBX_Door_Elevator1) (Math|Vector|MakeVector 0.0 (Math|Float|Lerp -158.0 -318.0 _open) 0.0) false false)
        (Transformation|SetRelativeLocation (Variables|Default|GetFBX_Door_Elevator) (Math|Vector|MakeVector 0.0 (Math|Float|Lerp -22.0 138.0 _open) 0.0) false false)))
    (else
      (Variables|Default|SetIsClosed true)
      (Timeline|open Reverse))))

(fn ConstructionScript)